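; BP_ExitDoor is a level exit that takes the first-person character to the next level once the door is opened.
; When the character enters its Box trigger while Opened is set, a DoOnce gate lets it fire a single time.
; It then shows a BP_Fade widget, plays its Fade animation, and after a short delay loads the level named by NextLevel.
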(event OnComponentBeginOverlap(Box)
  (params (OverlappedComponent :type Primitive%20Component%20Object%20Reference) (OtherActor :type Actor%20Object%20Reference) (OtherComp :type Primitive%20Component%20Object%20Reference) (OtherBodyIndex :type Integer) (bFromSweep :type Boolean) (SweepResult :type Hit%20Result%20Structure%20%28by%20ref%29))
  (Utilities|Casting|CastToBP_FirstPersonCharacter OtherActor)
  (if (Variables|Default|GetOpened)
    (Utilities|FlowControl|DoOnce false
      (:Completed
        (bind _returnvalue (UserInterface|CreateWidget "/Game/Spikes/BP_Fade.BP_Fade_C"))
        (UserInterface|Viewport|AddtoViewport _returnvalue 0)
        (UserInterface|Animation|PlayAnimation _returnvalue (Variables|/Game/Spikes/BP_Fade.BP_Fade_C|GetFade _returnvalue) 0.0 1 "Forward" 1.0 false)
        (Utilities|FlowControl|Delay 0.25)
        (Game|OpenLevel(byName) (Variables|Default|GetNext%20Level))))))

(fn ConstructionScript)