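; BP_Gem is a spinning collectible that the first-person character picks up to unlock the exit door.
; Each gem increments GemsNeeded in the GemUI widget after a zero-length delay on BeginPlay, using the widget text as the counter.
; First overlap increments GemsCollected, opens BP_ExitDoor and recolors it once both counts match.
; Pickup also flashes the UI, activates sounds, and hides the gem before delayed destruction.
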(event OnComponentBeginOverlap(Box)
  (params (OverlappedComponent :type Primitive%20Component%20Object%20Reference) (OtherActor :type Actor%20Object%20Reference) (OtherComp :type Primitive%20Component%20Object%20Reference) (OtherBodyIndex :type Integer) (bFromSweep :type Boolean) (SweepResult :type Hit%20Result%20Structure%20%28by%20ref%29))
  (Utilities|Casting|CastToBP_FirstPersonCharacter OtherActor)
  (Utilities|FlowControl|DoOnce false
    (:Completed
      (bind _foundwidgets (Widget|GetAllWidgetsOfClass "/Game/Collectibles/GemUI.GemUI_C" true))
      (Rendering|Components|TextRender|SetText (Variables|/Game/Collectibles/GemUI.GemUI_C|GetGemsCollected (Utilities|Array|Get(acopy) _foundwidgets)) (Utilities|Text|ToText(Integer) (+ (Math|Conversions|ToInteger(Byte) (Utilities|String|ToString(Text) (Class|TextBlock|GetText (Variables|/Game/Collectibles/GemUI.GemUI_C|GetGemsCollected (Utilities|Array|Get(acopy) _foundwidgets))))) 1)))
      (if (Utilities|Enum|Equal(Enum) (Class|TextBlock|GetText (Variables|/Game/Collectibles/GemUI.GemUI_C|GetGemsCollected (Utilities|Array|Get(acopy) _foundwidgets))) (Class|TextBlock|GetText (Variables|/Game/Collectibles/GemUI.GemUI_C|GetGemsNeeded (Utilities|Array|Get(acopy) _foundwidgets))))
        (bind _outactors (Actor|GetAllActorsOfClass "/Game/Collectibles/BP_ExitDoor.BP_ExitDoor_C"))
        (Variables|/Game/Collectibles/BP_ExitDoor.BP_ExitDoor_C|SetOpened (Utilities|Array|Get(acopy) _outactors) true)
        (Rendering|Material|SetMaterial (Variables|/Game/Collectibles/BP_ExitDoor.BP_ExitDoor_C|GetDoor (Utilities|Array|Get(acopy) _outactors)) 0 "/Game/Platform/Pink.Pink"))
      (UserInterface|Animation|PlayAnimation (Utilities|Array|Get(acopy) _foundwidgets) (Variables|/Game/Collectibles/GemUI.GemUI_C|GetFlash (Utilities|Array|Get(acopy) _foundwidgets)) 0.0 1 "Forward" 1.0 false)
      (Components|Activation|Activate (Variables|Default|GetGemSound2) false)
      (Rendering|SetActorHiddenInGame true)
      (Utilities|FlowControl|Delay 5.0)
      (Actor|DestroyActor))))

(event EventBeginPlay
  (Utilities|FlowControl|Sequence
    (:then_0
      (bind _newtrack_0 (Timeline|Rotation Play)
        (:Update
          (Transformation|SetWorldRotation (Variables|Default|GetGem) (Math|Rotator|MakeRotator 0.0 _newtrack_0 _newtrack_0) false false))))
    (:then_1
      (Utilities|FlowControl|Delay 0.0)
      (bind _foundwidgets (Widget|GetAllWidgetsOfClass "/Game/Collectibles/GemUI.GemUI_C" true))
      (Rendering|Components|TextRender|SetText (Variables|/Game/Collectibles/GemUI.GemUI_C|GetGemsNeeded (Utilities|Array|Get(acopy) _foundwidgets)) (Utilities|Text|ToText(Integer) (+ (Math|Conversions|ToInteger(Byte) (Utilities|String|ToString(Text) (Class|TextBlock|GetText (Variables|/Game/Collectibles/GemUI.GemUI_C|GetGemsNeeded (Utilities|Array|Get(acopy) _foundwidgets))))) 1))))))

(fn ConstructionScript)